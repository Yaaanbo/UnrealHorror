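; BP_Enemy is a horror-game enemy that chases the player on sight and ends the game on contact.
; PawnSensing starts AIMoveTo toward the seen pawn, while a retriggerable delay stops its movement two seconds after the last sighting.
; A capsule hit on the first-person character fires once, calling GameOver on the game instance, disabling player input, fading out the approach sound and playing a sting.
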(event `self.PawnSensing.OnSeePawn`
  (params (Pawn :type "Pawn Object Reference"))
  ;[0 0 0] AI Vision
  (`|ExecutionSequence`
    (:`then_0`
      (`|AIMoveTo` self (0.0 0.0 0.0) Pawn))
    (:`then_1`
      (`KismetSystemLibrary.RetriggerableDelay` 2.0)
      (`MovementComponent.StopMovementImmediately` (`self.CharacterMovement`)))))

(event `self.CapsuleComponent.OnComponentHit`
  (params (HitComponent :type "PrimitiveComponent Object Reference") (OtherActor :type "Actor Object Reference") (OtherComp :type "PrimitiveComponent Object Reference") (NormalImpulse :type "Vector Structure") (Hit :type "HitResult Structure (by ref)"))
  (bind _asbp_first_person_character (cast `/Game/FirstPerson/Blueprints/BP_FirstPersonCharacter` OtherActor))
  (bind _asbp_game_instance (cast `/Game/HorrorCourse/Blueprints/BP_GameInstance` (`GameplayStatics.GetGameInstance`)))
  (`/Engine/EditorBlueprintResources/StandardMacros.DoOnce` false
    (:`Completed`
      (`/Game/HorrorCourse/Blueprints/BP_GameInstance.Game Over` _asbp_game_instance)
      (`self.DisableInput` _asbp_first_person_character null)
      (`AudioComponent.AdjustVolume` (`self.SC_EnemyApproaching`) 2.0 0.0 "Linear")
      (`GameplayStatics.PlaySound2D` "/Game/HorrorCourse/Assets/Audio/Horror_sting.Horror_sting" 1.0 1.0 0.0 null null))))

(fn `UserConstructionScript`)