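; BP_InteractableObject is a collectible pickup actor that shows an interaction prompt when the player is near it.
; It creates a WBP_Interactable widget on BeginPlay and adds or removes it from the viewport as BP_FirstPersonCharacter begins or ends overlap.
; Its OnPickUp event increments the collectible count through BP_GameInstance's AddCollectibleItem, then destroys the actor.
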(event `/Game/HorrorCourse/Blueprints/BPI_Interactable.OnPickUp`
  (bind _asbp_game_instance (cast `/Game/HorrorCourse/Blueprints/BP_GameInstance` (`GameplayStatics.GetGameInstance`)))
  (`/Game/HorrorCourse/Blueprints/BP_GameInstance.Add Collectible Item` _asbp_game_instance)
  (`self.K2_DestroyActor`))

(event `self.ReceiveBeginPlay`
  (bind _returnvalue (`|CreateWidget` "/Game/HorrorCourse/UI/WBP_Interactable.WBP_Interactable_C")))

(event `self.ReceiveActorBeginOverlap`
  (params (OtherActor :type "Actor Object Reference"))
  (cast `/Game/FirstPerson/Blueprints/BP_FirstPersonCharacter` OtherActor)
  (`UserWidget.AddToViewport` (stale `self.ReceiveBeginPlay` _returnvalue) 0))

(event `self.ReceiveActorEndOverlap`
  (params (OtherActor :type "Actor Object Reference"))
  (cast `/Game/FirstPerson/Blueprints/BP_FirstPersonCharacter` OtherActor)
  (`Widget.RemoveFromParent` (stale `self.ReceiveBeginPlay` _returnvalue)))

(fn `UserConstructionScript`)